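; Combat arena actor that spawns enemies and can enclose the fight with four toggleable walls.
; On BeginPlay it spawns one BP_Enemy per spawn point entry at randomly picked, possibly repeated points, passing itself as a reference, then hides the walls.
; ActivateWalls restores wall visibility and collision.
; CheckIfEnemies1, uncalled by the live graph here, decrements the enemy count and at zero hides the walls and clears the player's IsInCombat flag.
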(event Custom|HideWalls
  (bind _round_5x1_05 (Variables|Default|Getround_5x1_05))
  ;[1 1 1] Hide Zone Walls
  (Development|SetHiddeninGame _round_5x1_05 true false)
  (Collision|SetCollisionEnabled _round_5x1_05 "NoCollision"))

(event Custom|ActivateWalls
  (bind _round_5x1_05 (Variables|Default|Getround_5x1_05))
  ;[1 1 1] Activate Zone Walls
  (Development|SetHiddeninGame _round_5x1_05 false false)
  (Collision|SetCollisionEnabled _round_5x1_05 "QueryAndPhysics"))

(event EventBeginPlay
  (bind _spawnpoints (Variables|Default|GetSpawnPoints))
  (bind _enemies (Variables|Default|GetEnemies))
  ;[1 1 1] BeginPlay & Spawn Enemies
  (for _array_element _spawnpoints
    (bind _returnvalue (Game|SpawnActorfromClass "/Game/Actors/BP_Enemy.BP_Enemy_C" (Math|Transform|MakeTransform (Transformation|GetActorLocation (.OutItem (Utilities|Array|Random _spawnpoints))) "0, 0, 0" "1.000000,1.000000,1.000000") "Undefined" 0 self 0))
    (Utilities|Array|Add _enemies _returnvalue)
    (Variables|Default|SetIndexValue (+ (Variables|Default|GetIndexValue) 1)))
  (Development|PrintString "Everything Spawned")
  (CallFunction|HideWalls)
  (Variables|Default|SetEnemiesCount (Utilities|Array|Length _enemies)))

(fn ConstructionScript)

(fn CheckifEnemies1
  (bind _result (Math|Integer|DecrementInt (Variables|Default|GetEnemiesCount))
    (:%20%20
      (if (<= _result 0)
        (CallFunction|HideWalls)
        (bind _asbp_third_person_character (Utilities|Casting|CastToBP_ThirdPersonCharacter (Game|GetPlayerCharacter 0)))
        (Variables|/Game/ThirdPerson/Blueprints/BP_ThirdPersonCharacter.BP_ThirdPersonCharacter_C|SetIsInCombat? _asbp_third_person_character false)
        (return)))))