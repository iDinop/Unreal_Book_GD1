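; BP_Dog is an AI-moved dog that heads for an objective waypoint and then removes itself, apparently as a guide to the objective.
; On BeginPlay a spawn flag gates ObjectiveLocalization, which issues AI MoveTo toward ObjectiveWaypoint if valid, then destroys the dog after a short delay.
; A timeline that would drive a material Fade parameter is present but unconnected, so it never runs.
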(event Custom|ObjectiveLocalization
  (bind _objectivewaypoint (Variables|Default|GetObjectiveWaypoint)
    (:then
      (AI|AIMoveTo self "0, 0, 0" _objectivewaypoint 5.0 false
        (:then
          _)
        (:OnSuccess
          _)
        (:OnFail
          _))
      (Utilities|FlowControl|Delay 3.0)
      (Variables|Default|SetAlreadySpawned? false)
      (Actor|DestroyActor))
    (:else)))

(event EventBeginPlay
  (if (not (Variables|Default|GetAlreadySpawned?))
    (Variables|Default|SetAlreadySpawned? true)
    (CallFunction|ObjectiveLocalization)))

(event Collision|EventActorBeginOverlap
  (params (OtherActor :type Actor%20Object%20Reference)))

(event EventTick
  (params (DeltaSeconds :type Float%20%28single-precision%29)))

(fn ConstructionScript)