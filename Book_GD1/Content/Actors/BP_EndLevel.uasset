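; BP_EndLevel is a trigger actor that lets the player finish the level once the boss is dead.
; Its box overlap stores the BP_ThirdPersonCharacter, enables input on the actor and opens a gate; leaving disables input and closes it.
; Inside, pressing IA_AttackorAxtion out of combat with BossHasBeenKilled set adds the W_EndLevel widget, switches to UI-only input and shows the mouse cursor.
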(event OnComponentBeginOverlap(Box)
  (params (OverlappedComponent :type Primitive%20Component%20Object%20Reference) (OtherActor :type Actor%20Object%20Reference) (OtherComp :type Primitive%20Component%20Object%20Reference) (OtherBodyIndex :type Integer) (bFromSweep :type Boolean) (SweepResult :type Hit%20Result%20Structure%20%28by%20ref%29))
  (bind _returnvalue (Game|GetPlayerController 0))
  (bind _asbp_third_person_character (Utilities|Casting|CastToBP_ThirdPersonCharacter OtherActor))
  (Variables|Default|SetCharREF _asbp_third_person_character)
  (Input|EnableInput (Game|GetPlayerController 0))
  (Utilities|FlowControl|Gate true) ; enters at Open
)

(event OnComponentEndOverlap(Box)
  (params (OverlappedComponent :type Primitive%20Component%20Object%20Reference) (OtherActor :type Actor%20Object%20Reference) (OtherComp :type Primitive%20Component%20Object%20Reference) (OtherBodyIndex :type Integer))
  (bind _returnvalue (Game|GetPlayerController 0))
  (bind _asbp_third_person_character (Utilities|Casting|CastToBP_ThirdPersonCharacter OtherActor))
  (Variables|Default|SetCharREF _asbp_third_person_character)
  (Input|DisableInput (Game|GetPlayerController 0))
  (Utilities|FlowControl|Gate true) ; enters at Close
)

(event Input|EnhancedActionEvents|EnhancedInputActionIA_AttackorAxtion
  (params (ActionValue :type Boolean) (ElapsedSeconds :type Float%20%28double-precision%29) (TriggeredSeconds :type Float%20%28double-precision%29) (InputAction :type Input%20Action%20Object%20Reference :default "/Game/ThirdPerson/Input/Actions/IA_AttackorAxtion.IA_AttackorAxtion"))
  (bind _returnvalue (Game|GetPlayerController 0))
  (:Started
    (if (not (Variables|/Game/ThirdPerson/Blueprints/BP_ThirdPersonCharacter.BP_ThirdPersonCharacter_C|GetIsInCombat? (stale OnComponentBeginOverlap(Box) _asbp_third_person_character)))
      (if (Variables|/Game/ThirdPerson/Blueprints/BP_ThirdPersonCharacter.BP_ThirdPersonCharacter_C|GetBossHasBeenKilled (Variables|Default|GetCharREF))
        (Utilities|FlowControl|Gate true
          (:Exit
            (bind _returnvalue_2 (UserInterface|CreateWidget "/Game/Widgets/W_EndLevel.W_EndLevel_C"))
            (UserInterface|Viewport|AddtoViewport _returnvalue_2 0)
            (Input|SetInputModeUIOnly _returnvalue 0 "DoNotLock" false)
            (Variables|/Script/Engine.PlayerController|SetbShowMouseCursor _returnvalue true)))))))

(fn ConstructionScript)