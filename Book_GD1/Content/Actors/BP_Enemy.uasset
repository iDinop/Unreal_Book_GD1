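; Enemy character that starts zone combat, chases the player and deals damage on contact.
; A player still inside its trigger after a timer activates the zone's walls and broadcasts combat start, which reveals the health bar.
; The chase re-issues AIMoveTo recursively, gated by detection, with Tick also re-triggering it on the enemy that started combat.
; Hits cause knockback and brief invincibility; death notifies the zone and grants experience.
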(event OnComponentBeginOverlap(CombatZone)
  (params (OverlappedComponent :type Primitive%20Component%20Object%20Reference) (OtherActor :type Actor%20Object%20Reference) (OtherComp :type Primitive%20Component%20Object%20Reference) (OtherBodyIndex :type Integer) (bFromSweep :type Boolean) (SweepResult :type Hit%20Result%20Structure%20%28by%20ref%29))
  ;[1 1 1] Start Zone Spawn Timer
  (bind _asbp_third_person_character (Utilities|Casting|CastToBP_ThirdPersonCharacter OtherActor))
  (Variables|Default|SetPlayerREF _asbp_third_person_character)
  (Variables|Default|SetIsInside true)
  (bind _returnvalue (Utilities|Time|SetTimerbyEvent (delegate Custom|CombatStart) 2.5)))

(event OnComponentEndOverlap(CombatZone)
  (params (OverlappedComponent :type Primitive%20Component%20Object%20Reference) (OtherActor :type Actor%20Object%20Reference) (OtherComp :type Primitive%20Component%20Object%20Reference) (OtherBodyIndex :type Integer))
  ;[1 1 1] Zone Trigger
  (Variables|Default|SetIsInside false))

(event OnComponentBeginOverlap(Detection)
  (params (OverlappedComponent :type Primitive%20Component%20Object%20Reference) (OtherActor :type Actor%20Object%20Reference) (OtherComp :type Primitive%20Component%20Object%20Reference) (OtherBodyIndex :type Integer) (bFromSweep :type Boolean) (SweepResult :type Hit%20Result%20Structure%20%28by%20ref%29))
  ;[1 1 1] Bool Check for Attack
  (Variables|Default|SetMustAttack true)
  (if (Variables|Default|GetMustAttack)
    (if (Variables|Default|GetZoneSpawned?)
      _)))

(event OnComponentBeginOverlap(CapsuleComponent)
  (params (OverlappedComponent :type Primitive%20Component%20Object%20Reference) (OtherActor :type Actor%20Object%20Reference) (OtherComp :type Primitive%20Component%20Object%20Reference) (OtherBodyIndex :type Integer) (bFromSweep :type Boolean) (SweepResult :type Hit%20Result%20Structure%20%28by%20ref%29))
  ;[1 1 1] Damages on collision
  (bind _asbp_third_person_character (Utilities|Casting|CastToBP_ThirdPersonCharacter OtherActor))
  (if (Variables|/Game/ThirdPerson/Blueprints/BP_ThirdPersonCharacter.BP_ThirdPersonCharacter_C|GetIsInCombat? _asbp_third_person_character)
    (if (Variables|/Game/ThirdPerson/Blueprints/BP_ThirdPersonCharacter.BP_ThirdPersonCharacter_C|GetIsRolling? _asbp_third_person_character)
      (if (not (Variables|/Game/ThirdPerson/Blueprints/BP_ThirdPersonCharacter.BP_ThirdPersonCharacter_C|GetInvincible _asbp_third_person_character))
        (Default|StopRolling _asbp_third_person_character)
        (Game|Damage|ApplyDamage _asbp_third_person_character 1.0 0 0 :!label _label))
      (elif (not (Variables|/Game/ThirdPerson/Blueprints/BP_ThirdPersonCharacter.BP_ThirdPersonCharacter_C|GetInvincible _asbp_third_person_character))
        (goto _label)))))

(event OnComponentEndOverlap(Detection)
  (params (OverlappedComponent :type Primitive%20Component%20Object%20Reference) (OtherActor :type Actor%20Object%20Reference) (OtherComp :type Primitive%20Component%20Object%20Reference) (OtherBodyIndex :type Integer))
  ;[1 1 1] Bool Check for Attack
  (bind _asbp_third_person_character (Utilities|Casting|CastToBP_ThirdPersonCharacter OtherActor))
  (if (== (Variables|/Script/Engine.Character|GetCapsuleComponent _asbp_third_person_character) OtherComp)
    (Variables|Default|SetMustAttack false)))

(event Custom|CombatStart
  ;[1 1 1] CombatStart
  (if (Variables|Default|GetIsInside)
    (Default|ActivateWalls (Variables|Default|GetCombatZoneREF))
    (Variables|/Game/ThirdPerson/Blueprints/BP_ThirdPersonCharacter.BP_ThirdPersonCharacter_C|SetIsInCombat? (Variables|Default|GetPlayerREF) true)
    (Variables|Default|SetZoneSpawned? true)
    (Default|CallCombatStarted (Variables|Default|GetCombatZoneREF) (Variables|Default|GetPlayerREF))
    (Utilities|Time|ClearandInvalidateTimerbyHandle (stale OnComponentBeginOverlap(CombatZone) _returnvalue))))

(event Custom|CombatMode
  ;[1 1 1] Combat Mode
  (if (Variables|Default|GetMustAttack)
    (AI|AIMoveTo self "0, 0, 0" (Variables|Default|GetPlayerREF) 5e+01 false
      (:OnSuccess
        _)
      (:OnFail
        _))
    (Utilities|FlowControl|Delay 0.25)
    (CallFunction|CombatMode)))

(event Custom|OnCombatStarted
  (params (PlayerREF :type BP%20Third%20Person%20Character%20Object%20Reference))
  (bind _w_healthbar (Variables|Default|GetW_HealthBar))
  (bind _returnvalue (UserInterface|GetWidget _w_healthbar))
  (Variables|Default|SetPlayerREF PlayerREF)
  (Variables|Default|SetMustAttack true)
  (CallFunction|CombatMode)
  (bind _asw_health_bar_enemy (Utilities|Casting|CastToW_HealthBar_Enemy _returnvalue))
  (Default|SetHealth _asw_health_bar_enemy (Variables|Default|GetcurrentHealth) (Variables|Default|GetmaxHealth))
  (Widget|SetVisibility _returnvalue "Visible"))

(event EventBeginPlay
  ;[1 1 1] Begin Play
  (Variables|Default|SetcurrentHealth (Variables|Default|GetmaxHealth))
  (Variables|Default|SetZoneSpawned? false)
  (EventDispatchers|BindEventtoCombatStarted (Variables|Default|GetCombatZoneREF) (delegate Custom|OnCombatStarted)))

(event EventTick
  (params (DeltaSeconds :type Float%20%28single-precision%29))
  ;[1 1 1] Chase Player
  (if (Variables|Default|GetZoneSpawned?)
    (for _array_element (Collision|GetOverlappingActors (Variables|Default|GetDetection) "/Game/ThirdPerson/Blueprints/BP_ThirdPersonCharacter.BP_ThirdPersonCharacter_C" :!class /Script/Engine.PrimitiveComponent)
      (Utilities|Casting|CastToBP_ThirdPersonCharacter _array_element)
      (CallFunction|CombatMode))))

(event Game|Damage|EventAnyDamage
  (params (Damage :type Float%20%28single-precision%29) (DamageType :type Damage%20Type%20Object%20Reference) (InstigatedBy :type Controller%20Object%20Reference) (DamageCauser :type Actor%20Object%20Reference))
  ;[1 1 1] Tale Damage & Destroy
  (if (not (Variables|Default|GetInvincible))
    (bind _output_get (Variables|Default|SetcurrentHealth (- (Variables|Default|GetcurrentHealth) Damage)))
    (Variables|Default|SetInvincible true)
    (Character|LaunchCharacter self "0.000000,350.000000,350.000000" true true)
    (if (<= _output_get 0.0)
      (Default|CheckifEnemies1 (Variables|Default|GetCombatZoneREF))
      (Default|Exp (Variables|Default|GetPlayerREF) (Variables|Default|GetExpGiven))
      (Actor|DestroyActor)
      (else
        (bind _asw_health_bar_enemy (Utilities|Casting|CastToW_HealthBar_Enemy (UserInterface|GetWidget (Variables|Default|GetW_HealthBar))))
        (Default|SetHealth _asw_health_bar_enemy (Variables|Default|GetcurrentHealth) (Variables|Default|GetmaxHealth))
        (Utilities|FlowControl|Delay 1.5)
        (Variables|Default|SetInvincible false)))))

(fn ConstructionScript)