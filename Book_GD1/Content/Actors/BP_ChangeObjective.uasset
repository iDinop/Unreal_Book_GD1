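; BP_ChangeObjective is a placeable objective trigger that advances the player's waypoint along a chain of linked objectives.
; On BeginPlay, the instance flagged as first objective sets itself as the third-person character's ObjectiveWaypoint.
; When a BP_ThirdPersonCharacter overlaps its CollisionBox, that character's waypoint switches to NextObjective, or clears when none is valid.
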(event OnComponentBeginOverlap(CollisionBox)
  (params (OverlappedComponent :type Primitive%20Component%20Object%20Reference) (OtherActor :type Actor%20Object%20Reference) (OtherComp :type Primitive%20Component%20Object%20Reference) (OtherBodyIndex :type Integer) (bFromSweep :type Boolean) (SweepResult :type Hit%20Result%20Structure%20%28by%20ref%29))
  (bind _asbp_third_person_character (Utilities|Casting|CastToBP_ThirdPersonCharacter OtherActor))
  (bind _nextobjective (Variables|Default|GetNextObjective)
    (:then
      (Variables|/Game/ThirdPerson/Blueprints/BP_ThirdPersonCharacter.BP_ThirdPersonCharacter_C|SetObjectiveWaypoint _asbp_third_person_character _nextobjective))
    (:else
      (Variables|/Game/ThirdPerson/Blueprints/BP_ThirdPersonCharacter.BP_ThirdPersonCharacter_C|SetObjectiveWaypoint _asbp_third_person_character 0))))

(event EventBeginPlay
  (if (Variables|Default|GetIsFirstObjective?)
    (bind _asbp_third_person_character (Utilities|Casting|CastToBP_ThirdPersonCharacter (Game|GetPlayerCharacter 0)))
    (Variables|/Game/ThirdPerson/Blueprints/BP_ThirdPersonCharacter.BP_ThirdPersonCharacter_C|SetObjectiveWaypoint _asbp_third_person_character self)))

(fn ConstructionScript)