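; BP_DialogueActor is an actor that presents one dialogue node with a text line and two player choices.
; OpenDialogue spawns W_Dialogue, passes it the text, answers, choice options and per-choice quest flags, then switches to UI-only input with a visible cursor.
; EndDialogue removes the widget and restores game input, while NextDialogue only removes the widget, leaving input in UI mode.
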(event Custom|OpenDialogue
  (bind _returnvalue (Game|GetPlayerController 0))
  (bind _returnvalue_2 (UserInterface|CreateWidget "/Game/Widgets/W_Dialogue.W_Dialogue_C"))
  (bind _output_get (Variables|Default|SetDialogueWidgetREF _returnvalue_2))
  (UserInterface|Viewport|AddtoViewport _output_get 0)
  (Variables|/Game/Widgets/W_Dialogue.W_Dialogue_C|SetDialogueActor (Variables|Default|GetDialogueWidgetREF) self)
  (Input|DisableInput _returnvalue)
  (Variables|/Script/Engine.PlayerController|SetbShowMouseCursor _returnvalue true)
  (Input|SetInputModeUIOnly (Game|GetPlayerController 0) (Variables|Default|GetDialogueWidgetREF) "DoNotLock" false)
  (Variables|/Script/UMG.TextBlock|SetText (Variables|/Game/Widgets/W_Dialogue.W_Dialogue_C|GetTextToShow (Variables|Default|GetDialogueWidgetREF)) (Variables|Default|GetTextToShow))
  (Variables|/Script/UMG.TextBlock|SetText (Variables|/Game/Widgets/W_Dialogue.W_Dialogue_C|GetChoice1Text (Variables|Default|GetDialogueWidgetREF)) (Variables|Default|GetAnswerText1))
  (Variables|/Script/UMG.TextBlock|SetText (Variables|/Game/Widgets/W_Dialogue.W_Dialogue_C|GetChoice2Text (Variables|Default|GetDialogueWidgetREF)) (Variables|Default|GetAnswerText2))
  (Variables|/Game/Widgets/W_Dialogue.W_Dialogue_C|SetOption1 (Variables|Default|GetDialogueWidgetREF) (Variables|Default|GetChoice1))
  (Variables|/Game/Widgets/W_Dialogue.W_Dialogue_C|SetOption2 (Variables|Default|GetDialogueWidgetREF) (Variables|Default|GetChoice2))
  (if (Variables|Default|GetChoice1Quest?)
    (Variables|/Game/Widgets/W_Dialogue.W_Dialogue_C|SetChoice1Quest? (Variables|Default|GetDialogueWidgetREF) true)
    (else
      (Variables|/Game/Widgets/W_Dialogue.W_Dialogue_C|SetChoice1Quest? (Variables|Default|GetDialogueWidgetREF) false)))
  (if (Variables|Default|GetChoice2Quest?)
    (Variables|/Game/Widgets/W_Dialogue.W_Dialogue_C|SetChoice2Quest? (Variables|Default|GetDialogueWidgetREF) true)
    (else
      (Variables|/Game/Widgets/W_Dialogue.W_Dialogue_C|SetChoice2Quest? (Variables|Default|GetDialogueWidgetREF) false))))

(event Custom|EndDialogue
  (bind _returnvalue (Game|GetPlayerController 0))
  (Widget|RemovefromParent (Variables|Default|GetDialogueWidgetREF))
  (Variables|Default|SetDialogueWidgetREF 0)
  (Input|EnableInput _returnvalue)
  (Variables|/Script/Engine.PlayerController|SetbShowMouseCursor _returnvalue false)
  (Input|SetInputModeGameOnly _returnvalue false))

(event Custom|NextDialogue
  (Widget|RemovefromParent (Variables|Default|GetDialogueWidgetREF))
  (Variables|Default|SetDialogueWidgetREF 0))

(fn ConstructionScript)